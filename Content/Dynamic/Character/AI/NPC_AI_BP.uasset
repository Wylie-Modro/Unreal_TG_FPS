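; AI controller for guard NPCs that runs the GuardBehaviour tree on the PatrolData blackboard.
; Perception updates skip actors tagged "Mates", setting the enemy key to player character 0 (not the sensed actor) on successful sensing, with a debug print, and clearing it otherwise.
; Each tick, the controlled Character_BP's aiming and shooting flags mirror whether the controller has a valid focus actor.
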(event `self.ReceiveBeginPlay`
  (bind _blackboardcomponent (`self.UseBlackboard` "/Game/Dynamic/Character/AI/PatrolData.PatrolData"))
  (set `self.BlackboardComp` _blackboardcomponent)
  (`self.RunBehaviorTree` "/Game/Dynamic/Character/AI/GuardBehaviour.GuardBehaviour"))

(event `self.ReceiveTick`
  (params (DeltaSeconds :type "Float (single-precision)"))
  (bind _returnvalue (`KismetSystemLibrary.IsValid` (`self.GetFocusActor`)))
  (bind _ascharacter_bp (cast `/Game/Dynamic/Character/Character_BP` (`self.K2_GetPawn`)))
  (set `/Game/Dynamic/Character/Character_BP.isAiming` _returnvalue _ascharacter_bp)
  (set `/Game/Dynamic/Character/Character_BP.isShooting` _returnvalue _ascharacter_bp))

(event `self.AIPerception.OnTargetPerceptionUpdated`
  (params (Actor :type "Actor Object Reference") (Stimulus :type "AIStimulus Structure"))
  (bind _blackboardcomp (`self.BlackboardComp`))
  (bind _enemykey (`self.EnemyKey`))
  (if (not (`self.ActorHasTag` Actor "Mates"))
    (bind _returnvalue (`AIPerceptionSystem.GetSenseClassForStimulus` Stimulus))
    (if (`.bSuccessfullySensed` (break `AIStimulus` Stimulus))
      (`BlackboardComponent.SetValueAsObject` _blackboardcomp _enemykey (`GameplayStatics.GetPlayerCharacter` 0))
      (`KismetSystemLibrary.PrintString` (`KismetStringLibrary.Concat_StrStr` (`KismetSystemLibrary.GetObjectName` (`self.K2_GetPawn`)) " " (`KismetSystemLibrary.GetClassDisplayName` _returnvalue) " " (`KismetSystemLibrary.GetObjectName` Actor)))
      (else
        (`BlackboardComponent.ClearValue` _blackboardcomp _enemykey)))))

(fn `UserConstructionScript`)