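; BP_Tile is one section of an infinite terrain, scattering randomized containers, canisters, boxes, sandbags and rocks via PlaceActors on BeginPlay.
; The player entering LockingVolume disables the barrier's collision; leaving it asks InfiniteTerrainGameMode to spawn another tile.
; Entering DestroyVolume destroys the tile, and GetAttachLocation exposes the Arrow transform as an attach point.
; LockBarrier, which restores collision with a red material, is never called here.
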(event `self.ReceiveBeginPlay`
  (`self.SpawnProps`))

(event `self.LockingVolume.OnComponentBeginOverlap`
  (params (OverlappedComponent :type "PrimitiveComponent Object Reference") (OtherActor :type "Actor Object Reference") (OtherComp :type "PrimitiveComponent Object Reference") (OtherBodyIndex :type Integer) (bFromSweep :type Boolean) (SweepResult :type "HitResult Structure (by ref)"))
  (`self.IsPlayerCharacter` OtherActor
    (:`true`
      (`self.UnlockBarrier`))))

(event `self.LockingVolume.OnComponentEndOverlap`
  (params (OverlappedComponent :type "PrimitiveComponent Object Reference") (OtherActor :type "Actor Object Reference") (OtherComp :type "PrimitiveComponent Object Reference") (OtherBodyIndex :type Integer))
  (`self.IsPlayerCharacter` OtherActor
    (:`true`
      (bind _asinfinite_terrain_game_mode (cast `/Game/Dynamic/InfiniteTerrainGameMode` (`GameplayStatics.GetGameMode`)))
      (`/Game/Dynamic/InfiniteTerrainGameMode.SpawnTile` _asinfinite_terrain_game_mode))))

(event `self.DestroyVolume.OnComponentBeginOverlap`
  (params (OverlappedComponent :type "PrimitiveComponent Object Reference") (OtherActor :type "Actor Object Reference") (OtherComp :type "PrimitiveComponent Object Reference") (OtherBodyIndex :type Integer) (bFromSweep :type Boolean) (SweepResult :type "HitResult Structure (by ref)"))
  (`self.IsPlayerCharacter` OtherActor
    (:`true`
      (`self.K2_DestroyActor`))))

(fn `GetAttachLocation`
  (returns (AttachTransform :type "Transform Structure"))
  (return (`SceneComponent.K2_GetComponentToWorld` (`self.Arrow`))))

(fn `LockBarrier`
  (`PrimitiveComponent.SetCollisionEnabled` (`self.Barrier`) "QueryAndPhysics")
  (`PrimitiveComponent.SetMaterial` (`self.Barrier`) 0 "/Game/Dynamic/Terrain/MI_Barrier_Red.MI_Barrier_Red"))

(fn `SpawnProps`
  (`self.PlaceActors` "/Game/Dynamic/Terrain/Props/BP_Container.BP_Container_C" 1 5 500 1.0 1.0)
  (`self.PlaceActors` "/Game/Dynamic/Terrain/Props/BP_Canister.BP_Canister_C" 2 12 80 0.5 1.5)
  (`self.PlaceActors` "/Game/Dynamic/Terrain/Props/BP_Box.BP_Box_C" 2 5 120 0.7 1.5)
  (`self.PlaceActors` "/Game/Dynamic/Terrain/Props/BP_SandBag.BP_SandBag_C" 3 8 100 0.8)
  (`self.PlaceActors` "/Game/Dynamic/Terrain/Props/BP_Rock01.BP_Rock01_C" 1 3 250 0.2 2.5)
  (`self.PlaceActors` "/Game/Dynamic/Terrain/Props/BP_Rock02.BP_Rock02_C" 1 3 250 0.2 2.5)
  (`self.PlaceActors` "/Game/Dynamic/Terrain/Props/BP_Rock03.BP_Rock03_C" 1 3 250300 0.2 2.5))

(fn `UnlockBarrier`
  (`PrimitiveComponent.SetCollisionEnabled` (`self.Barrier`) "NoCollision"))

(fn `UserConstructionScript`)