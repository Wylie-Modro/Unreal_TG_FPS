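; Terrain tile for an infinite terrain mode, gated by a barrier and exposing its Arrow transform as an attach location.
; Player entry into LockingVolume disables barrier collision; exit restores it, applies the red material and asks InfiniteTerrainGameMode to spawn a tile.
; The tile destroys itself when the player overlaps DestroyVolume.
; An IsPlayerCharacter macro limits all triggers to player 0's character.
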(event `self.ReceiveBeginPlay`)

(event `self.LockingVolume.OnComponentBeginOverlap`
  (params (OverlappedComponent :type "PrimitiveComponent Object Reference") (OtherActor :type "Actor Object Reference") (OtherComp :type "PrimitiveComponent Object Reference") (OtherBodyIndex :type Integer) (bFromSweep :type Boolean) (SweepResult :type "HitResult Structure (by ref)"))
  (`self.IsPlayerCharacter` OtherActor
    (:`true`
      (`self.UnlockBarrier`))))

(event `self.LockingVolume.OnComponentEndOverlap`
  (params (OverlappedComponent :type "PrimitiveComponent Object Reference") (OtherActor :type "Actor Object Reference") (OtherComp :type "PrimitiveComponent Object Reference") (OtherBodyIndex :type Integer))
  (`self.IsPlayerCharacter` OtherActor
    (:`true`
      (`self.LockBarrier`)
      (bind _asinfinite_terrain_game_mode (cast `/Game/Dynamic/InfiniteTerrainGameMode` (`GameplayStatics.GetGameMode`)))
      (`/Game/Dynamic/InfiniteTerrainGameMode.SpawnTile` _asinfinite_terrain_game_mode))))

(event `self.DestroyVolume.OnComponentBeginOverlap`
  (params (OverlappedComponent :type "PrimitiveComponent Object Reference") (OtherActor :type "Actor Object Reference") (OtherComp :type "PrimitiveComponent Object Reference") (OtherBodyIndex :type Integer) (bFromSweep :type Boolean) (SweepResult :type "HitResult Structure (by ref)"))
  (`self.IsPlayerCharacter` OtherActor
    (:`true`
      (`self.K2_DestroyActor`))))

(fn `GetAttachLocation`
  (returns (AttachTransform :type "Transform Structure"))
  (return (`SceneComponent.K2_GetComponentToWorld` (`self.Arrow`))))

(fn `LockBarrier`
  (`PrimitiveComponent.SetCollisionEnabled` (`self.Barrier`) "QueryAndPhysics")
  (`PrimitiveComponent.SetMaterial` (`self.Barrier`) 0 "/Game/Dynamic/Terrain/RedBarrier.RedBarrier"))

(fn `UnlockBarrier`
  (`PrimitiveComponent.SetCollisionEnabled` (`self.Barrier`) "NoCollision"))

(fn `UserConstructionScript`)